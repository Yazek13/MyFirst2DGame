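; BP_Hero is a player character that moves along the world X axis in side-scroller style, with a dash.
; The Move axis drives movement input, while Tick snaps control yaw to face left or right from the sign of X velocity.
; Both are gated by IsMovementLock.
; Holding Dash raises max walk speed and the RunPlayeRate variable, and releasing it restores both.
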(event EventBeginPlay)

(event Collision|EventActorBeginOverlap
  (params (OtherActor :type Actor%20Object%20Reference)))

(event EventTick
  (params (DeltaSeconds :type Float%20%28single-precision%29))
  (bind _returnvalue (Pawn|GetController))
  (bind _returnvalue_2 (Pawn|GetController))
  ;[1 1 1] Character Rotation
  (if (not (Variables|Default|GetisMovementLock))
    (Math|Float|CompareFloat (.x (Variables|/Script/Engine.MovementComponent|GetVelocity (Variables|Character|GetCharacterMovement))) 0.0
      (:>
        ;;[1 1 1] Right
        (Utilities|IsValid _returnvalue_2
          (:Is%20Valid
            (Pawn|SetControlRotation _returnvalue_2 (Math|Rotator|MakeRotator 0.0 0.0 0.0)))))
      (:<
        ;;[1 1 1] Left
        (Utilities|IsValid _returnvalue
          (:Is%20Valid
            (Pawn|SetControlRotation _returnvalue (Math|Rotator|MakeRotator 0.0 0.0 1.8e+02))))))))

(event Input|ActionEvents|InputActionDash
  (params (Key :type Key%20Structure :default "None"))
  ;[1 1 1] Dash
  (:Pressed
    (Variables|Default|SetRunPlayeRate 1.5)
    (Variables|/Script/Engine.CharacterMovementComponent|SetMaxWalkSpeed (Variables|Character|GetCharacterMovement) 1e+03))
  (:Released
    (Variables|Default|SetRunPlayeRate 1.0)
    (Variables|/Script/Engine.CharacterMovementComponent|SetMaxWalkSpeed (Variables|Character|GetCharacterMovement) 6e+02)))

(event Input|AxisEvents|InputAxisMove
  (params (AxisValue :type Float%20%28single-precision%29))
  ;[1 1 1] Forward
  (if (not (Variables|Default|GetisMovementLock))
    (Pawn|Input|AddMovementInput "1.000000,0.000000,0.000000" AxisValue false)))

(fn ConstructionScript)